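; Flipbook enemy that chases the tail of the player's line of friends, held in the GameMode's TremzinhoDaAlegria array.
; Reaching the tail, or hitting another non-player member, destroys the last friend, retargets all enemies and kills itself.
; Hitting the player ahead of friends kills only itself; each death requests a replacement spawn.
; Catching a lone player triggers enemy win animations, costs a life, then reloads the level or opens GameOverScreen.
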(event `Enemy Death`
  ;[1 1 1] Sends order for a new spawn, set on death animation, and after delay, kill this enemy
  (bind _asrecn_play_game_mode_bp (cast `/Game/Blueprints/RecnPlay_GameMode_BP` (`GameplayStatics.GetGameMode`)))
  (`/Game/Blueprints/RecnPlay_GameMode_BP.Spawn Enemy At Closest Spawning Point` _asrecn_play_game_mode_bp)
  (set `self.IsDying` true)
  (`PaperFlipbookComponent.SetFlipbook` (`self.Sprite`) "/Game/Extras/Paper2D/G_Death.G_Death")
  (`PrimitiveComponent.SetCollisionEnabled` (`self.CapsuleComponent`) "NoCollision")
  (`KismetSystemLibrary.Delay` (`self.DeathAnimationTimer`))
  (`self.K2_DestroyActor`))

(event `self.ReceiveHit`
  (params (MyComp :type "PrimitiveComponent Object Reference") (Other :type "Actor Object Reference") (OtherComp :type "PrimitiveComponent Object Reference") (bSelfMoved :type Boolean) (HitLocation :type "Vector Structure") (HitNormal :type "Vector Structure") (NormalImpulse :type "Vector Structure") (Hit :type "HitResult Structure (by ref)"))
  ;[1 1 1] If enemy hit an actor that is not it's target, kill it if it's a friend but not the player
  (if (not (`self.IsDying`))
    (bind _asrecn_play_game_mode_bp (cast `/Game/Blueprints/RecnPlay_GameMode_BP` (`GameplayStatics.GetGameMode`)))
    (bind _tremzinhodaalegria (`/Game/Blueprints/RecnPlay_GameMode_BP.TremzinhoDaAlegria` _asrecn_play_game_mode_bp))
    (if (!= (`|GetArrayItem` _tremzinhodaalegria (`KismetArrayLibrary.Array_LastIndex` _tremzinhodaalegria)) Other)
      (bind _aspawn (cast `Pawn` Other))
      (if (`KismetArrayLibrary.Array_Contains` _tremzinhodaalegria _aspawn)
        (if (`self.ActorHasTag` Other "Player")
          ;[1 1 1] If it's a player, only kill self
          (`self.Enemy Death`)
          (else
            ;[1 1 1] It's not a player; kill that friend and self
            (`self.Kill Last Friend of Line And Enemy`)))))))

(event `Chase Actor`
  ;[1 1 1] Make enemy chase last character of the array
  (if (not (`self.IsDying`))
    (bind _asrecn_play_game_mode_bp (cast `/Game/Blueprints/RecnPlay_GameMode_BP` (`GameplayStatics.GetGameMode`)))
    (bind _tremzinhodaalegria (`/Game/Blueprints/RecnPlay_GameMode_BP.TremzinhoDaAlegria` _asrecn_play_game_mode_bp))
    (`|AIMoveTo` self (0.0 0.0 0.0) (`|GetArrayItem` _tremzinhodaalegria (`KismetArrayLibrary.Array_LastIndex` _tremzinhodaalegria))
      (:`OnSuccess`
        (`self.Kill Last Friend of Line And Enemy`)))))

(event `Kill Last Friend of Line And Enemy`
  (bind _returnvalue (`GameplayStatics.GetPlayerPawn` 0))
  ;[1 1 1] Kills last friend of array, kill self, and re-spawn
  (if (not (`self.IsDying`))
    (bind _asrecn_play_game_mode_bp (cast `/Game/Blueprints/RecnPlay_GameMode_BP` (`GameplayStatics.GetGameMode`)))
    (bind _tremzinhodaalegria (`/Game/Blueprints/RecnPlay_GameMode_BP.TremzinhoDaAlegria` _asrecn_play_game_mode_bp))
    (if (== (`KismetArrayLibrary.Array_Length` _tremzinhodaalegria) 1)
      ;[1 1 1] If last friend in line is the player (length = 1), disable player input, make all enemies have win animation, and after delay, reduce player lives by 1
      (`self.SetActorHiddenInGame` _returnvalue true)
      (`self.DisableInput` _returnvalue (`GameplayStatics.GetPlayerController` 0))
      (if (not (`self.HasWon`))
        (bind _returnvalue_2 (`AddComponent|NODE_AddAudioComponent-0`))
        (`AudioComponent.Play` _returnvalue_2 0.0)
        (set `self.HasWon` true))
      (bind _outactors (`GameplayStatics.GetAllActorsOfClass` "Enemy_BP_C"))
      (for _array_element _outactors
        (`PaperFlipbookComponent.SetFlipbook` (`PaperCharacter.Sprite` _array_element) "/Game/Extras/Paper2D/G_Win.G_Win"))
      (`KismetSystemLibrary.Delay` (`self.LaughingTimer`))
      (bind _asgame_instance_bp (cast `/Game/Blueprints/GameInstance_BP` (`GameplayStatics.GetGameInstance`)))
      (bind _result (`/Engine/EditorBlueprintResources/StandardMacros.DecrementInt` (`/Game/Blueprints/GameInstance_BP.PlayerLives` _asgame_instance_bp))
        (:`  `
          (if (<= _result 0)
            ;[1 1 1] If player lives is now <= 0, game over
            (`GameplayStatics.OpenLevel` "GameOverScreen")
            (else
              ;[1 1 1] If player still has lives, reload level
              (bind _returnvalue_3 (`GameplayStatics.GetCurrentLevelName` true))
              (`GameplayStatics.OpenLevel` (`KismetStringLibrary.Conv_StringToName` _returnvalue_3))))))
      (else
        (bind _output (`|GetArrayItem` _tremzinhodaalegria (`KismetArrayLibrary.Array_LastIndex` _tremzinhodaalegria)))
        ;[1 1 1] If last friend in line is not player, destroy it and self
        (`self.K2_DestroyActor` _output)
        (`KismetArrayLibrary.Array_RemoveItem` _tremzinhodaalegria _output)
        (bind _asgame_instance_bp_2 (cast `/Game/Blueprints/GameInstance_BP` (`GameplayStatics.GetGameInstance`)))
        (`/Engine/EditorBlueprintResources/StandardMacros.IncrementInt` (`/Game/Blueprints/GameInstance_BP.UnsavedFriends` _asgame_instance_bp_2)
          (:`  `
            (bind _outactors_2 (`GameplayStatics.GetAllActorsOfClass` "Enemy_BP_C"))
            (for _array_element_2 _outactors_2
              (`self.Chase Actor` _array_element_2))
            (`self.Enemy Death`)))))))

(fn `UserConstructionScript`)