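; Game mode that runs enemy spawning for each level and starts the friends array with the player pawn.
; On BeginPlay it reads the level's spawn delay and enemy cap from the game instance, adds UnsavedFriends to the cap, then resets that counter.
; A looping timer, followed by an equal Delay, spawns an Enemy_BP at the cached spawn point closest to the player while under the cap, then starts its chase.
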(event `self.ReceiveBeginPlay`
  (bind _tremzinhodaalegria (`self.TremzinhoDaAlegria`))
  (`|ExecutionSequence`
    (:`then_0`
      ;[1 1 1] Determine current level index and maximum amount of enemies per level
      (bind _asgame_instance_bp (cast `/Game/Blueprints/GameInstance_BP` (`GameplayStatics.GetGameInstance`)))
      (set `self.MaxEnemyCount` (+ (`/Game/Blueprints/GameInstance_BP.UnsavedFriends` _asgame_instance_bp) (`BlueprintMapLibrary.Map_Find` (`/Game/Blueprints/GameInstance_BP.Map_LevelIndex_To_MaxEnemyCount` _asgame_instance_bp) (`/Game/Blueprints/GameInstance_BP.IndexCurrentLevel` _asgame_instance_bp))))
      (set `/Game/Blueprints/GameInstance_BP.UnsavedFriends` 0 _asgame_instance_bp)
      ;[1 1 1] Determine spawn timer according to level
      (bind _asgame_instance_bp_2 (cast `/Game/Blueprints/GameInstance_BP` (`GameplayStatics.GetGameInstance`)))
      (set `self.EnemySpawnDelay` (`BlueprintMapLibrary.Map_Find` (`/Game/Blueprints/GameInstance_BP.Map_LevelIndex_To_SpawnTimer` _asgame_instance_bp_2) (`/Game/Blueprints/GameInstance_BP.IndexCurrentLevel` _asgame_instance_bp_2))))
    (:`then_1`
      ;[1 1 1] Add Player to array of friends
      (`KismetArrayLibrary.Array_Clear` _tremzinhodaalegria)
      (`KismetArrayLibrary.Array_Add` _tremzinhodaalegria (`GameplayStatics.GetPlayerPawn` 0)))
    (:`then_2`
      ;[1 1 1] Make array containing the position of all Enemy Spawn Points
      (bind _outactors (`GameplayStatics.GetAllActorsOfClass` "/Game/Blueprints/EnemySpawnPoint.EnemySpawnPoint_C"))
      (for _array_element _outactors
        (`KismetArrayLibrary.Array_Add` (`self.SpawnPoints`) (`self.K2_GetActorLocation` _array_element)))
      ;[1 1 1] Create timer to keep looping Spawn Enemy event
      (bind _returnvalue (`KismetSystemLibrary.K2_SetTimerDelegate` (delegate `Spawn Enemy At Closest Spawning Point`) (`self.EnemySpawnDelay`) true))
      (set `self.Timer` _returnvalue))))

(event `Spawn Enemy At Closest Spawning Point`
  (bind _spawnpoints (`self.SpawnPoints`))
  ;[1 1 1] Only Spawn enemy if enemy count is lower than max enemy count
  (bind _outactors (`GameplayStatics.GetAllActorsOfClass` "/Game/Blueprints/Enemy_BP.Enemy_BP_C"))
  (if (< (`KismetArrayLibrary.Array_Length` _outactors) (`self.MaxEnemyCount`))
    ;[1 1 1] Create array containing distances from each spawn point to player, and find the index of the lowest distance
    (`KismetSystemLibrary.Delay` (`self.EnemySpawnDelay`))
    (`KismetArrayLibrary.Array_Resize` (`self.SpawnPointsDistancesToPlayer`) (`KismetArrayLibrary.Array_Length` _spawnpoints))
    (for (_array_element _array_index) _spawnpoints
      (`KismetArrayLibrary.Array_Set` (`self.SpawnPointsDistancesToPlayer`) _array_index (`KismetMathLibrary.VSize` (- _array_element (`self.K2_GetActorLocation` (`GameplayStatics.GetPlayerPawn` 0))))))
    ;[1 1 1] Spawn enemy at the closest spawn point and make it chase friends
    (bind _returnvalue (`|SpawnActorFromClass` "/Game/Blueprints/Enemy_BP.Enemy_BP_C" (`KismetMathLibrary.Conv_VectorToTransform` (`|GetArrayItem` (`self.SpawnPoints`) (`KismetMathLibrary.MinOfFloatArray` (`self.SpawnPointsDistancesToPlayer`)))) "AdjustIfPossibleButAlwaysSpawn" "OverrideRootScale" null null))
    (`/Game/Blueprints/Enemy_BP.Chase Actor` _returnvalue)))

(fn `UserConstructionScript`)